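; Player controller test Blueprint that maps debug keys to cursor visibility and to shooting on a NewBlueprint actor.
; BeginPlay caches the first NewBlueprint found in the level, while the E and K keys look it up again to call StartShoot and Shoot.
; Keys 1 and 2 show and hide the mouse cursor.
; Unwired nodes that set GrabMode and IsCameraLock never run.
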(event `self.ReceiveBeginPlay`
  (bind _outactors (`GameplayStatics.GetAllActorsOfClass` "/Game/Models/NewBlueprint.NewBlueprint_C"))
  (set `self.NewVar_0` (`|GetArrayItem` _outactors)))

(event `Key|SpaceBar`
  (params (Key :type "Key Structure")))

(event `Key|One`
  (params (Key :type "Key Structure"))
  (:`Pressed`
    (set `PlayerController.bShowMouseCursor` true (`GameplayStatics.GetPlayerController` 0))))

(event `Key|Two`
  (params (Key :type "Key Structure"))
  (:`Pressed`
    (set `PlayerController.bShowMouseCursor` false (`GameplayStatics.GetPlayerController` 0))))

(event `Key|E`
  (params (Key :type "Key Structure"))
  (:`Pressed`
    (bind _outactors (`GameplayStatics.GetAllActorsOfClass` "/Game/Models/NewBlueprint.NewBlueprint_C"))
    (`/Game/Models/NewBlueprint.StartShoot` (`|GetArrayItem` _outactors))))

(event `Key|K`
  (params (Key :type "Key Structure"))
  (:`Pressed`
    (bind _outactors (`GameplayStatics.GetAllActorsOfClass` "/Game/Models/NewBlueprint.NewBlueprint_C"))
    (`/Game/Models/NewBlueprint.Shoot` (`|GetArrayItem` _outactors))))

(fn `UserConstructionScript`)